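; BP_Villain is an enemy actor that fires projectiles at random intervals and can be destroyed by projectile hits.
; From BeginPlay, a Delay wired back onto itself repeatedly spawns BP_Villain_Projectile at the Ponta component's position and rotation, printing the loop index.
; The surrounding ForLoop does not limit the shot count, as the cycle repeats indefinitely.
; Overlapping an actor of exactly the Projectile class plays an explosion sound and destroys the villain.
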(event Collision|EventActorBeginOverlap
  (params (OtherActor :type Actor%20Object%20Reference))
  ;[1 1 1] Destruction
  (if (== "/Game/VRTemplate/Blueprints/Projectile.Projectile_C" (Utilities|GetClass OtherActor))
    (Audio|PlaySound2D "/Game/StarterContent/Audio/Explosion02.Explosion02" 1.0 1.0 0.0 0 0)
    (Actor|DestroyActor)))

(event EventBeginPlay
  (bind _ponta (Variables|Default|GetPonta))
  (for _index (range 0 10)
    (Utilities|FlowControl|Delay (* (Math|Float|MultiplybyPi (Math|Random|RandomFloat)) 1e+01) :!label _label)
    (Game|SpawnActorfromClass "/Game/Blueprints/BP_Villain_Projectile.BP_Villain_Projectile_C" (Math|Transform|MakeTransform (Transformation|GetWorldLocation _ponta) (Transformation|GetWorldRotation _ponta)) "Undefined" self 0)
    (Development|PrintString (Utilities|String|ToString(Integer) _index))
    (goto _label)))

(fn ConstructionScript)